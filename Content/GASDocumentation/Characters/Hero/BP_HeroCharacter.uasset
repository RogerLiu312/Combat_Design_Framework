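; Hero character Blueprint for a Gameplay Ability System project, handling sprint input and on-screen debug output.
; Sprint press calls SwitchByPressAbility, which checks PlayerState's ability system tags and sends either the cancel or activate gameplay event.
; PressAndHoldAbility is an unused, identical copy; in both, cancel events carry PayloadForActivate and activate events PayloadForCancel.
; Tick prints owned gameplay tags and movement rotation rate every frame.
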(event `self.ReceiveBeginPlay`)

(event `self.ReceiveActorBeginOverlap`
  (params (OtherActor :type "Actor Object Reference")))

(event `self.ReceiveTick`
  (params (DeltaSeconds :type "Float (single-precision)"))
  (for _array_element (`BlueprintGameplayTagLibrary.BreakGameplayTagContainer` (`GameplayTagAssetInterface.GetOwnedGameplayTags` (`AbilitySystemBlueprintLibrary.GetAbilitySystemComponent` self)))
    (`KismetSystemLibrary.PrintString` (`KismetStringLibrary.Conv_NameToString` (`BlueprintGameplayTagLibrary.GetTagName` _array_element)) true true (struct :`G` 0.66 :`B` 1.0 :`A` 1.0) DeltaSeconds))
  (`KismetSystemLibrary.PrintString` (`KismetStringLibrary.Conv_RotatorToString` (`CharacterMovementComponent.RotationRate` (`self.CharacterMovement`))) true true (struct :`G` 0.66 :`B` 1.0 :`A` 1.0) DeltaSeconds))

(event `InputAction|Sprint`
  (params (Key :type "Key Structure"))
  (:`Pressed`
    (`self.Switch_By_Press_Ability` (struct :`TagName` "Ability.Sprint") (struct :`TagName` "Ability.CancelSprint"))))

(fn `Press_And_Hold_Ability`
  (params (Ability_Tag :type "GameplayTag Structure") (Ability_Cancel_Tag :type "GameplayTag Structure") (Payload_For_Activate :type "GameplayEventData Structure") (Payload_For_Cancel :type "GameplayEventData Structure"))
  (if (`BlueprintGameplayTagLibrary.HasTag` (`GameplayTagAssetInterface.GetOwnedGameplayTags` (`AbilitySystemBlueprintLibrary.GetAbilitySystemComponent` (`self.PlayerState`))) Ability_Tag)
    (`AbilitySystemBlueprintLibrary.SendGameplayEventToActor` self Ability_Cancel_Tag Payload_For_Activate)
    (else
      (`AbilitySystemBlueprintLibrary.SendGameplayEventToActor` self Ability_Tag Payload_For_Cancel))))

(fn `Switch_By_Press_Ability`
  (params (Ability_Tag :type "GameplayTag Structure") (Ability_Cancel_Tag :type "GameplayTag Structure") (Payload_For_Activate :type "GameplayEventData Structure") (Payload_For_Cancel :type "GameplayEventData Structure"))
  (if (`BlueprintGameplayTagLibrary.HasTag` (`GameplayTagAssetInterface.GetOwnedGameplayTags` (`AbilitySystemBlueprintLibrary.GetAbilitySystemComponent` (`self.PlayerState`))) Ability_Tag)
    (`AbilitySystemBlueprintLibrary.SendGameplayEventToActor` self Ability_Cancel_Tag Payload_For_Activate)
    (else
      (`AbilitySystemBlueprintLibrary.SendGameplayEventToActor` self Ability_Tag Payload_For_Cancel))))

(fn `UserConstructionScript`)